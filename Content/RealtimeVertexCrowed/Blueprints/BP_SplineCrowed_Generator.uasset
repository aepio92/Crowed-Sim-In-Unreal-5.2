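; Spline-based crowd generator that lines static meshes along a spline at construction time.
; The construction script divides spline length by Spacing and adds a separate static mesh component at each step, in local space.
; Each component faces the next sample point and gets a random mesh from the Meshes array, picked with the Seed random stream for repeatable layouts.
; The event graph has no active logic.
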(fn `GetLocationAtIndex`
  (params (Index :type Integer))
  (returns (Location :type "Vector Structure"))
  (return (`SplineComponent.GetLocationAtDistanceAlongSpline` (`self.Spline`) (* Index (`self.Spacing`)) "Local")))

(fn `UserConstructionScript`
  (bind _meshes (`self.Meshes`))
  (bind _output_get (set `self.No of Instances` (`KismetMathLibrary.FFloor` (/ (`SplineComponent.GetSplineLength` (`self.Spline`)) (`self.Spacing`)))))
  (for _index (range (+ _output_get 1))
    (bind _location (`self.GetLocationAtIndex` _index))
    (bind _returnvalue (`AddComponent|NODE_AddStaticMeshComponent-0` :`RelativeTransform` (`KismetMathLibrary.MakeTransform` _location (`KismetMathLibrary.MakeRotFromX` (- (`self.GetLocationAtIndex` (+ _index 1)) _location)))))
    (`StaticMeshComponent.SetStaticMesh` _returnvalue (`|GetArrayItem` _meshes (`KismetMathLibrary.RandomIntegerInRangeFromStream` (`self.Seed`) 0 (- (`KismetArrayLibrary.Array_Length` _meshes) 1))))))